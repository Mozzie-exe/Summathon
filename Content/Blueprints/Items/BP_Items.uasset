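; BP_Items is an interactable item actor that highlights with an overlay material when looked at and can be picked up by Char.
; On interact, currency adds to Money, updates the HUD counter and destroys itself.
; Other items add ItemDetails to the inventory, then either attach to HoldPoint with physics off or are destroyed if something is already held.
; OnDropped detaches the item, restores collision and physics, and throws it along the camera's forward vector.
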(event `SetItemOverlayActive`
  (params (`IsLookedAt?` :type Boolean))
  (bind _staticmesh (`self.StaticMesh`))
  (if `IsLookedAt?`
    (`MeshComponent.SetOverlayMaterial` _staticmesh "/Game/Materials/M_HighlightOutline_Inst.M_HighlightOutline_Inst")
    (else
      (`MeshComponent.SetOverlayMaterial` _staticmesh null))))

(event `self.Interact`
  (params (Interactor :type "Actor Object Reference"))
  (bind _staticmesh (`self.StaticMesh`))
  (bind (_itemname _itemtype _weight _value) (break `ItemData` (`self.ItemDetails`)))
  (bind _aschar (cast `/Game/Blueprints/Char` Interactor))
  (if (`|EnumEquality` _itemtype "Currency")
    (bind _output_get (set `ChacterScript.Money` (+ (`ChacterScript.Money` _aschar) _value) _aschar))
    (`TextBlock.SetText` (`/Game/UIElements/W_HUD.Txt_MoneyCounter` (`/Game/Blueprints/Char.HudReference` _aschar)) (`|FormatText` "{Para} $" (`KismetTextLibrary.Conv_IntToText` _output_get)))
    (`self.K2_DestroyActor`)
    (elif (`KismetSystemLibrary.IsValid` (`/Game/Blueprints/Char.HeldActor` _aschar))
      (`/Game/Blueprints/Char.AddItem` _aschar (`self.ItemDetails`) 1)
      (`self.K2_DestroyActor`)
      (else
        (set `/Game/Blueprints/Char.HeldActor` self _aschar)
        (`PrimitiveComponent.SetSimulatePhysics` _staticmesh false)
        (`PrimitiveComponent.SetCollisionEnabled` _staticmesh "NoCollision")
        (`self.K2_AttachToComponent` (`/Game/Blueprints/Char.HoldPoint` _aschar) "None" "SnapToTarget" "SnapToTarget" "KeepWorld" false)
        (`/Game/Blueprints/Char.AddItem` _aschar (`self.ItemDetails`) 1)))))

(fn `OnDropped`
  (bind _staticmesh (`self.StaticMesh`))
  (`self.K2_DetachFromActor` "KeepWorld" "KeepWorld" "KeepWorld")
  (`PrimitiveComponent.SetCollisionEnabled` _staticmesh "QueryAndPhysics")
  (`PrimitiveComponent.SetSimulatePhysics` _staticmesh true)
  (`PrimitiveComponent.AddImpulse` _staticmesh (* (`self.GetActorForwardVector` (`GameplayStatics.GetPlayerCameraManager` 0)) 500) "None" false))

(fn `UserConstructionScript`)