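; BP_Elma is a pickup item that a Char can hold, add to its inventory and throw.
; Interact sets it as the character's HeldActor, disables the Cube's physics and collision, and snaps it to HoldPoint.
; It also appends ItemDetails to the Inventory and prints every item name.
; OnDropped detaches it, restores physics and collision, and launches it along the camera's forward vector, leaving the inventory untouched.
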(event `InteractInterface.Interact`
  (params (Interactor :type "Actor Object Reference"))
  (bind _cube (`self.Cube`))
  (bind _aschar (cast `/Game/Blueprints/Char` Interactor))
  (set `/Game/Blueprints/Char.HeldActor` self _aschar)
  (`PrimitiveComponent.SetSimulatePhysics` _cube false)
  (`PrimitiveComponent.SetCollisionEnabled` _cube "NoCollision")
  (`self.K2_AttachToComponent` (`/Game/Blueprints/Char.HoldPoint` _aschar) "None" "SnapToTarget" "SnapToTarget" "SnapToTarget" false)
  (bind _inventory (`/Game/Blueprints/Char.Inventory` _aschar))
  (`KismetArrayLibrary.Array_Add` _inventory (`self.ItemDetails`))
  (for _array_element _inventory
    (`KismetSystemLibrary.PrintText` (`.ItemName` (break `ItemData` _array_element)))))

(fn `OnDropped`
  (bind _cube (`self.Cube`))
  (`self.K2_DetachFromActor` "KeepWorld" "KeepWorld" "KeepWorld")
  (`PrimitiveComponent.SetCollisionEnabled` _cube "QueryAndPhysics")
  (`PrimitiveComponent.SetSimulatePhysics` _cube true)
  (`PrimitiveComponent.AddImpulse` _cube (* (`self.GetActorForwardVector` (`GameplayStatics.GetPlayerCameraManager` 0)) 500) "None" false))

(fn `UserConstructionScript`)