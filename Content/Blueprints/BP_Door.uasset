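; Interactive hinged door Blueprint that swings open and closed when its Interact event fires.
; A FlipFlop alternately plays and reverses a timeline, whose alpha interpolates the Pivot component's yaw between closed and open angles.
; A collision box shows the interaction text on the overlapping Char's HUD reference and hides it when the overlap ends.
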(event `InteractInterface.Interact`
  (params (Interactor :type "Actor Object Reference"))
  (`/Engine/EditorBlueprintResources/StandardMacros.FlipFlop`
    (:`A`
      (bind (_direction _alpha) (`Timeline|DoorTimeLine` :!label _label)
        (:`Update`
          (`SceneComponent.K2_SetRelativeRotation` (`self.pivot`) (`KismetMathLibrary.MakeRotator` 0.0 0.0 (`KismetMathLibrary.Lerp` 0.0 100.0 _alpha)) false false))))
    (:`B`
      (goto _label :!via `Reverse`))))

(event `self.boxcollision.OnComponentBeginOverlap`
  (params (OverlappedComponent :type "PrimitiveComponent Object Reference") (OtherActor :type "Actor Object Reference") (OtherComp :type "PrimitiveComponent Object Reference") (OtherBodyIndex :type Integer) (bFromSweep :type Boolean) (SweepResult :type "HitResult Structure (by ref)"))
  (bind _aschar (cast `/Game/Blueprints/Char` OtherActor))
  (`Widget.SetVisibility` (`/Game/UIElements/W_HUD.InteractionText` (`/Game/Blueprints/Char.HudReference` _aschar)) "Visible"))

(event `self.boxcollision.OnComponentEndOverlap`
  (params (OverlappedComponent :type "PrimitiveComponent Object Reference") (OtherActor :type "Actor Object Reference") (OtherComp :type "PrimitiveComponent Object Reference") (OtherBodyIndex :type Integer))
  (bind _aschar (cast `/Game/Blueprints/Char` OtherActor))
  (`Widget.SetVisibility` (`/Game/UIElements/W_HUD.InteractionText` (`/Game/Blueprints/Char.HudReference` _aschar)) "Hidden"))

(fn `UserConstructionScript`)