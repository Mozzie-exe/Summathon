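; BP_Para is an interactable money pickup for the Char character.
; Interact sets it as the character's HeldActor; if its ItemDetails type is Currency, it adds the value to Money, updates the HUD counter and destroys itself.
; OnDropped detaches it, restores collision and physics on its Money component, and throws it along the camera's forward vector.
; Older hold-point attach and inventory-slot logic remains in the graph but never runs.
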(event `self.Interact`
  (params (Interactor :type "Actor Object Reference"))
  (bind (_itemname _itemtype _weight _value) (break `ItemData` (`self.ItemDetails`)))
  (bind _aschar (cast `/Game/Blueprints/Char` Interactor))
  (set `/Game/Blueprints/Char.HeldActor` self _aschar)
  (if (`|EnumEquality` _itemtype "Currency")
    (bind _output_get (set `ChacterScript.Money` (+ (`ChacterScript.Money` _aschar) _value) _aschar))
    (`TextBlock.SetText` (`/Game/W_HUD.Txt_MoneyCounter` (`/Game/Blueprints/Char.HudReference` _aschar)) (`KismetTextLibrary.Conv_IntToText` _output_get))
    (`self.K2_DestroyActor`)))

(fn `OnDropped`
  (bind _money (`self.money`))
  (`self.K2_DetachFromActor` "KeepWorld" "KeepWorld" "KeepWorld")
  (`PrimitiveComponent.SetCollisionEnabled` _money "QueryAndPhysics")
  (`PrimitiveComponent.SetSimulatePhysics` _money true)
  (`PrimitiveComponent.AddImpulse` _money (* (`self.GetActorForwardVector` (`GameplayStatics.GetPlayerCameraManager` 0)) 500) "None" false))

(fn `UserConstructionScript`)