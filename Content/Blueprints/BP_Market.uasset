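; BP_Market is an interactable market that opens and closes a shop window for the player character.
; Interact registers the market on the interacting Char if its inventory is closed, then creates W_MarketWindow if none exists and switches to game-and-UI input with a cursor.
; CloseMarket removes the widget, restores game-only input and clears the character's market reference and inventory-open flag.
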(event `CloseMarket`
  (bind _returnvalue (`GameplayStatics.GetPlayerController` 0))
  (bind _aschar (cast `/Game/Blueprints/Char` (`GameplayStatics.GetPlayerCharacter` 0)))
  (`Widget.RemoveFromParent` (`self.ActiveMarketWidgetReference`))
  (`WidgetBlueprintLibrary.SetInputMode_GameOnly` _returnvalue)
  (set `PlayerController.bShowMouseCursor` false _returnvalue)
  (set `/Game/Blueprints/Char.ActiveMarketReference` null _aschar)
  (set `/Game/Blueprints/Char.InventoryOpen` false _aschar)
  (`KismetSystemLibrary.PrintString` "Market closed")
  (set `self.ActiveMarketWidgetReference` null))

(event `InteractInterface.Interact`
  (params (Interactor :type "Actor Object Reference"))
  (bind _returnvalue (`GameplayStatics.GetPlayerController` 0))
  (bind _aschar (cast `/Game/Blueprints/Char` Interactor))
  (if (not (`/Game/Blueprints/Char.InventoryOpen` _aschar))
    (set `/Game/Blueprints/Char.ActiveMarketReference` self _aschar)
    (`/Engine/EditorBlueprintResources/StandardMacros.IsValid` (`self.ActiveMarketWidgetReference`)
      (:`Is Not Valid`
        (bind _returnvalue_2 (`|CreateWidget` "/Game/UIElements/W_MarketWindow.W_MarketWindow_C"))
        (bind _output_get (set `self.ActiveMarketWidgetReference` _returnvalue_2))
        (`UserWidget.AddToViewport` _output_get 0)
        (`WidgetBlueprintLibrary.SetInputMode_GameAndUIEx` _returnvalue _returnvalue_2 "DoNotLock" false true)
        (set `PlayerController.bShowMouseCursor` true _returnvalue)
        (`KismetSystemLibrary.PrintString` "widget olusturuldu")))))

(fn `UserConstructionScript`)